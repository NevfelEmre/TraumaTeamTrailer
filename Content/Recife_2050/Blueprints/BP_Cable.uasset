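; BP_Cable is a spline-driven cable actor that lays a chosen static mesh along an editable spline.
; The construction script adds one spline mesh component per segment between consecutive spline points, attached to the spline and bent using each point's local position and tangent.
; Mesh and forward axis come from variables, and each segment gets query-only collision.
; It has no active runtime logic.
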(event EventBeginPlay)

(event Collision|EventActorBeginOverlap
  (params (OtherActor :type Actor%20Object%20Reference)))

(event EventTick
  (params (DeltaSeconds :type Float%20%28single-precision%29)))

(fn ConstructionScript
  (bind _spline_nova (Variables|Default|GetSpline_Nova))
  (for _index (range 0 (- (Spline|GetNumberOfSplinePoints _spline_nova) 2))
    (bind _returnvalue (AddComponent|AddSplineMeshComponent false))
    (Components|StaticMesh|SetStaticMesh _returnvalue (Variables|Default|GetStaticMesh))
    (SplineMesh|SetForwardAxis _returnvalue (Variables|Default|GetforwardAxis) true)
    (Transformation|AttachComponentToComponent _returnvalue _spline_nova "None" "KeepRelative" "KeepRelative" "KeepRelative" true)
    (SplineMesh|SetStartandEnd _returnvalue (Spline|GetLocationatSplinePoint _spline_nova _index "Local") (Spline|GetTangentatSplinePoint _spline_nova _index "Local") (Spline|GetLocationatSplinePoint _spline_nova (+ _index 1) "Local") (Spline|GetTangentatSplinePoint _spline_nova (+ _index 1) "Local") true :!class /Script/Engine.SplineMeshComponent)
    (Collision|SetCollisionEnabled _returnvalue "QueryOnly")))